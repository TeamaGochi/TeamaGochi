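; AR player pawn that finds a detected plane to place the test character pawn on.
; Until scanning succeeds, Tick line-traces tracked AR geometry from screen center about once a second, storing the first hit if it is a valid plane.
; Each attempt calls the OnPlaneScanningDone dispatcher, bound at BeginPlay.
; SpawnCharacterOnPlane spawns BP_TESTPAWN_Won at the stored plane's center and keeps a reference.
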(event EventTick
  (params (DeltaSeconds :type Float%20%28single-precision%29))
  (Utilities|FlowControl|Sequence
    (:then_0
      ;[0.15 0.15 0.15 0.5] 바닥만들기
      (if (not (Variables|GameState|GetScanningIsDone))
        ;;[0.15 0.15 0.15 0.5] 누적시간이 1초보다 클 경우
        (bind _output_get (Variables|Timer|SetShowPlaneTimer (+ (Utilities|Time|GetWorldDeltaSeconds) (Variables|Timer|GetShowPlaneTimer))))
        (if (> _output_get 1.0)
          (Variables|Timer|SetShowPlaneTimer 0.0)
          (bind _result (CallFunction|SearchforSpawnCharacterPlaneCandidate))
          (Variables|GameState|SetScanningIsDone _result)
          (Default|CallOnPlaneScanningDone))))))

(event EventBeginPlay
  (EventDispatchers|BindEventtoOnPlaneScanningDone (EventDispatchers|CreateEvent :!event SpawnCharacteronPlane)))

(fn ConstructionScript)

(fn SearchforSpawnCharacterPlaneCandidate
  ;[0.15 0.15 0.15 0.5] AR Geometry 에 대한 레이트레이싱
  (bind _returnvalue (Class|ARBlueprintLibrary|LineTraceTrackedObjects (CallFunction|GetScreenCenterPosition) false false))
  (Math|Integer|CompareInt (Utilities|Array|Length _returnvalue)
    (:>
      (bind _asarplane_geometry (Utilities|Casting|CastToARPlaneGeometry (Class|ARTraceResultLibrary|GetTrackedGeometry (Utilities|Array|Get(acopy) _returnvalue))))
      (if (Utilities|IsValid _asarplane_geometry)
        (Variables|Default|SetPlaneGeometryToSpawn _asarplane_geometry)
        (return true)
        (else
          (return false))))))

(fn GetScreenCenterPosition
  (bind _returnvalue (Game|GetPlayerController 0))
  (bind (_sizex _sizey) (HUD|GetViewportSize _returnvalue))
  (return (* (Math|Vector2D|MakeVector2D (Math|Conversions|ToFloat(Integer) _sizex) (Math|Conversions|ToFloat(Integer) _sizey)) 0.5)))

(fn SpawnCharacteronPlane
  (bind _planegeometrytospawn (Variables|Default|GetPlaneGeometryToSpawn)
    (:then
      (bind _returnvalue (Game|SpawnActorfromClass "/Game/TeamaGochi/WonYuChan/Pawn/BP_TESTPAWN_Won.BP_TESTPAWN_Won_C" (Math|Transform|MakeTransform (Class|ARPlaneGeometry|GetCenter _planegeometrytospawn) "0, 0, 0" "1.000000,1.000000,1.000000") "Undefined" "MultiplyWithRoot" 0 0))
      (Variables|Character|SetSpawnedCharacter _returnvalue))
    (:else)))