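; Player state for a Tamagotchi-style pet game, tracking Hungry and Sleepy values plus eating and sleeping flags.
; The GM_TeamaGochi timer event lowers both stats, and each change updates the StateWidget through PC_TemaGochi's MainUI.
; Feed and GotoBed restore the stats, while named timers clear flags set by Feed and UpdateSleepy.
; The both-stats-empty check has no action yet, and Tick prints Hungry for debugging.
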(event Custom|TimerEvent
  (CallFunction|UpdateHungry)
  (CallFunction|UpdateSleepy)
  (if (Math|Float|NearlyEqual(Float) (+ (Variables|Default|GetSleepy) (Variables|Default|GetHungry)) 0.0 0.001)
    _))

(event EventBeginPlay
  (bind _asgm_teama_gochi (Utilities|Casting|CastToGM_TeamaGochi (Game|GetGameMode)))
  (EventDispatchers|BindEventtoTimerEvent _asgm_teama_gochi (delegate Custom|TimerEvent)))

(event EventTick
  (params (DeltaSeconds :type Float%20%28single-precision%29))
  (Development|PrintString (Utilities|String|ToString(Float) (Variables|Default|GetHungry))))

(fn ConstructionScript)

(fn UpdateHungry
  (Variables|Default|SetHungry (- (Variables|Default|GetHungry) 2e+01))
  (bind _aspc_tema_gochi (Utilities|Casting|CastToPC_TemaGochi (Game|GetPlayerController)))
  (Default|UpdateHungry (Variables|/Game/TeamaGochi/WonYuChan/UI/WB_MainUI.WB_MainUI_C|GetStateWidget (Variables|/Game/TeamaGochi/MainGame/PC_TemaGochi.PC_TemaGochi_C|GetMainUI _aspc_tema_gochi)) (Variables|Default|GetHungry))
  (Development|PrintString "Hungry Down"))

(fn UpdateSleepy
  (Variables|Default|SetSleepy (- (Variables|Default|GetSleepy) 1e+01))
  (bind _aspc_tema_gochi (Utilities|Casting|CastToPC_TemaGochi (Game|GetPlayerController)))
  (Default|UpdateSleepy (Variables|/Game/TeamaGochi/WonYuChan/UI/WB_MainUI.WB_MainUI_C|GetStateWidget (Variables|/Game/TeamaGochi/MainGame/PC_TemaGochi.PC_TemaGochi_C|GetMainUI _aspc_tema_gochi)) (Variables|Default|GetSleepy))
  (Variables|Default|SetIsSleeping true)
  (Utilities|Time|SetTimerbyFunctionName 0 "DelaySleeping" 3.0))

(fn Feed
  (Variables|Default|SetHungry (Math|Float|Clamp(Float) (+ (Variables|Default|GetHungry) 3e+01) 0.0 1e+02))
  (bind _aspc_tema_gochi (Utilities|Casting|CastToPC_TemaGochi (Game|GetPlayerController)))
  (Default|UpdateHungry (Variables|/Game/TeamaGochi/WonYuChan/UI/WB_MainUI.WB_MainUI_C|GetStateWidget (Variables|/Game/TeamaGochi/MainGame/PC_TemaGochi.PC_TemaGochi_C|GetMainUI _aspc_tema_gochi)) (Variables|Default|GetHungry))
  (Variables|Default|SetIsEating true)
  (Utilities|Time|SetTimerbyFunctionName 0 "DelayEating" 0.0))

(fn GotoBed
  (Variables|Default|SetSleepy 1e+02)
  (bind _aspc_tema_gochi (Utilities|Casting|CastToPC_TemaGochi (Game|GetPlayerController)))
  (Default|UpdateSleepy (Variables|/Game/TeamaGochi/WonYuChan/UI/WB_MainUI.WB_MainUI_C|GetStateWidget (Variables|/Game/TeamaGochi/MainGame/PC_TemaGochi.PC_TemaGochi_C|GetMainUI _aspc_tema_gochi)) (Variables|Default|GetSleepy))
  (Variables|Default|SetIsSleeping true))

(fn DelayEating
  (Variables|Default|SetIsEating false))

(fn DelaySleeping
  (Variables|Default|SetIsSleeping false))