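; Player controller for a Tamagotchi-style pet game that opens the character selection screen when play begins.
; BeginPlay creates the Widget_SelectCharacter widget for player 0 and adds it to the viewport.
; An older main UI creation chain is left disconnected, so the MainUI variable is never set.
; FeedCharacter, SleepCharacter and CleanCharacter are empty stubs for pet-care actions, and Tick is disabled.
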(event EventTick
  (params (DeltaSeconds :type Float%20%28single-precision%29))
  (|CallParentFunction DeltaSeconds) ; This node is disabled and will not be called.\nDrag off pins to build functionality.
)

(event EventBeginPlay
  ;[0.15 0.15 0.15 0.5] 캐릭터 ui 생성
  (|CallParentFunction)
  (bind _returnvalue (UserInterface|CreateWidget "/Game/TeamaGochi/KoHyeWon/Widget_SelectCharacter.Widget_SelectCharacter_C" (Game|GetPlayerController 0)))
  (UserInterface|Viewport|AddtoViewport _returnvalue 0))

(fn ConstructionScript
  (|CallParentFunction))

(fn FeedCharacter)

(fn SleepCharacter)

(fn CleanCharacter)