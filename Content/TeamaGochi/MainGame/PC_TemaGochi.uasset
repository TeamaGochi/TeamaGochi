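; Player controller for the TeamaGochi main game that owns the main UI and drives its startup screens.
; On BeginPlay it creates the main widget, shows the character selection panel and caches the possessed BP_PlayerPawn.
; Tick polls the pawn's CharacterSpawned flag and, through a DoOnce, hides the spawn loading widget once the character has spawned.
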(event EventBeginPlay
  ;[0.15 0.15 0.15 0.5] 메인 위젯 생성
  (bind _returnvalue (UserInterface|CreateWidget "/Game/TeamaGochi/MainGame/Widget/MainUIWidget.MainUIWidget_C" (Game|GetPlayerController 0)))
  (bind _output_get (Variables|Widget|SetWB_MainUI _returnvalue))
  (UserInterface|Viewport|AddtoViewport _output_get 0)
  ;[0.15 0.15 0.15 0.5] 캐릭 선택창
  (Widget|SetVisibility (Variables|/Game/TeamaGochi/MainGame/Widget/MainUIWidget.MainUIWidget_C|GetWidget_SelectCharacter (Variables|Widget|GetWB_MainUI)) "Visible")
  (bind _asbp_player_pawn (Utilities|Casting|CastToBP_PlayerPawn (Pawn|GetControlledPawn)))
  (Variables|PlayerPawn|SetBP%20Player%20Pawn _asbp_player_pawn))

(event EventTick
  (params (DeltaSeconds :type Float%20%28single-precision%29))
  (Utilities|FlowControl|Sequence
    (:then_0
      ;[0.15 0.15 0.15 0.5] 캐릭터가 스폰되면 스폰로딩 위젯 숨기기
      (if (Variables|/Game/TeamaGochi/MainGame/BP_PlayerPawn.BP_PlayerPawn_C|GetbCharacterSpawned (Variables|PlayerPawn|GetBP%20Player%20Pawn))
        (Utilities|FlowControl|DoOnce false
          (:Completed
            (Widget|SetVisibility (Variables|/Game/TeamaGochi/MainGame/Widget/MainUIWidget.MainUIWidget_C|GetSpawnLoadingWidget (Variables|Widget|GetWB_MainUI)) "Hidden")))))))

(fn ConstructionScript)