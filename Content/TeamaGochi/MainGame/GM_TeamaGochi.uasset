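; GM_TeamaGochi is the TeamaGochi game mode that runs an accelerated game clock and fires a periodic timer event.
; Tick accumulates time at ten times real speed and detects each in-game minute boundary, roughly every six real seconds.
; When the player pawn has a valid spawned character, it calls TimerEvent through a DoOnce, which resets after a short delay to prevent repeat firing within the same boundary.
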(event EventTick
  (params (DeltaSeconds :type Float%20%28single-precision%29))
  (bind _output_get (Variables|Default|SetTotalSecond (+ (* DeltaSeconds 1e+01) (Variables|Default|GetTotalSecond))))
  (if (== (Math|Float|Floor (Math|Float|%(Float) _output_get 6e+01)) 0)
    (bind _asbp_player_pawn (Utilities|Casting|CastToBP_PlayerPawn (Pawn|GetControlledPawn (Game|GetPlayerController 0))))
    (Variables|/Game/TeamaGochi/MainGame/BP_PlayerPawn.BP_PlayerPawn_C|GetSpawnedCharacter _asbp_player_pawn
      (:then
        ;[0.15 0.15 0.15 0.5] Comment
        (Utilities|FlowControl|DoOnce false :!label _label
          (:Completed
            (Utilities|FlowControl|Sequence
              (:then_0
                (Default|CallTimerEvent))
              (:then_1
                (Utilities|FlowControl|Delay 1.1)
                (goto _label Reset))))))
      (:else))))

(fn ConstructionScript)