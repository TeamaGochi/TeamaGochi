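; BP_TMPlayerState is the player state for a Tamagotchi-style game, holding the pet's Hungry and Sleepy stats and its current state.
; A timer event bound through GM_TeamaGochi lowers both stats without clamping, and every change is pushed to the controller's state widget.
; Feed raises Hungry, spawning a poop widget at a random screen position when full, while GotoBed refills Sleepy.
; Both actions set a temporary state that a timer resets.
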(event Custom|TimerEvent
  ;[0.15 0.15 0.15 0.5] Widet Binding
  (Widget|WidgetUpdateHungry)
  (Widget|WidgetUpdateSleepy))

(event EventBeginPlay
  (Variables|Default|SetHungry 1e+02)
  (Variables|Default|SetSleepy 1e+02)
  ;[0.15 0.15 0.15 0.5] Widet Binding
  (bind _asgm_teama_gochi (Utilities|Casting|CastToGM_TeamaGochi (Game|GetGameMode)))
  (EventDispatchers|BindEventtoTimerEvent _asgm_teama_gochi (delegate Custom|TimerEvent)))

(fn ConstructionScript)

(fn WidgetUpdateHungry
  (Variables|Default|SetHungry (- (Variables|Default|GetHungry) 2e+01))
  (bind _aspc_tema_gochi (Utilities|Casting|CastToPC_TemaGochi (Game|GetPlayerController)))
  (Default|UpdateHungry (Variables|/Game/TeamaGochi/MainGame/Widget/MainUIWidget.MainUIWidget_C|GetStateWidget (Variables|/Game/TeamaGochi/MainGame/PC_TemaGochi.PC_TemaGochi_C|GetWB_MainUI _aspc_tema_gochi)) (Variables|Default|GetHungry)))

(fn WidgetUpdateSleepy
  (Variables|Default|SetSleepy (- (Variables|Default|GetSleepy) 1e+01))
  (bind _aspc_tema_gochi (Utilities|Casting|CastToPC_TemaGochi (Game|GetPlayerController)))
  ;[0.15 0.15 0.15 0.5] Comment
  (Default|UpdateSleepy (Variables|/Game/TeamaGochi/MainGame/Widget/MainUIWidget.MainUIWidget_C|GetStateWidget (Variables|/Game/TeamaGochi/MainGame/PC_TemaGochi.PC_TemaGochi_C|GetWB_MainUI _aspc_tema_gochi)) (Variables|Default|GetSleepy)))

(fn Feed
  (bind _returnvalue (Viewport|GetViewportSize))
  ;[0.15 0.15 0.15 0.5] 배고픔 수치 증가
  (Variables|Default|SetHungry (Math|Float|Clamp(Float) (+ (Variables|Default|GetHungry) 3e+01) 0.0 1e+02))
  ;[0.15 0.15 0.15 0.5] 위젯 수치 업데이트
  (bind _aspc_tema_gochi (Utilities|Casting|CastToPC_TemaGochi (Game|GetPlayerController)))
  (Default|UpdateHungry (Variables|/Game/TeamaGochi/MainGame/Widget/MainUIWidget.MainUIWidget_C|GetStateWidget (Variables|/Game/TeamaGochi/MainGame/PC_TemaGochi.PC_TemaGochi_C|GetWB_MainUI _aspc_tema_gochi)) (Variables|Default|GetHungry))
  ;[0.15 0.15 0.15 0.5] 상태변화
  (CallFunction|ChangeCurrentState "NewEnumerator1")
  ;[0.15 0.15 0.15 0.5] 배변 프로세스
  (if (>= (Variables|Default|GetHungry) 1e+02)
    (bind _returnvalue_2 (UserInterface|CreateWidget "/Game/TeamaGochi/MainGame/Widget/PoopWidget.PoopWidget_C" 0 0 0))
    (UserInterface|Viewport|AddtoViewport _returnvalue_2 0)
    (Class|UserWidget|SetPositioninViewport _returnvalue_2 (Math|Vector2D|MakeVector2D (Math|Random|RandomFloatinRange 0.0 (- (.x _returnvalue) 1e+02)) (Math|Random|RandomFloatinRange 3e+02 (- (.y _returnvalue) 3e+02))) true)))

(fn GotoBed
  ;[0.15 0.15 0.15 0.5] 졸림 수치 설정
  (Variables|Default|SetSleepy 1e+02)
  ;[0.15 0.15 0.15 0.5] 위젯 수치 업데이트
  (bind _aspc_tema_gochi (Utilities|Casting|CastToPC_TemaGochi (Game|GetPlayerController)))
  (Default|UpdateSleepy (Variables|/Game/TeamaGochi/MainGame/Widget/MainUIWidget.MainUIWidget_C|GetStateWidget (Variables|/Game/TeamaGochi/MainGame/PC_TemaGochi.PC_TemaGochi_C|GetWB_MainUI _aspc_tema_gochi)) (Variables|Default|GetSleepy))
  ;[0.15 0.15 0.15 0.5] 상태변화
  (CallFunction|ChangeCurrentState "NewEnumerator2"))

(fn ChangeCurrentState
  (params (New%20State :type E_State%20Enum :default "NewEnumerator0"))
  ;[0.15 0.15 0.15 0.5] 상태변화
  (bind _asbp_tmplayer_state (Utilities|Casting|CastToBP_TMPlayerState (Game|GetPlayerState 0)))
  (Variables|BP_TMPlayerState_C|SetCurrentState _asbp_tmplayer_state New%20State)
  (Utilities|Time|SetTimerbyFunctionName 0 "ResetState" 3.0))

(fn ResetState
  (Variables|Default|SetCurrentState "NewEnumerator0"))